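; Saw hazard that moves along a path and damages the player on contact.
; The construction script builds an InterpToMovement path from two relative location variables, with the Speed variable setting the movement duration, so a higher value means slower travel.
; A sphere overlap casts the other actor to Player_BP and applies one point of damage.
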(event `self.Sphere.OnComponentBeginOverlap`
  (params (OverlappedComponent :type "PrimitiveComponent Object Reference") (OtherActor :type "Actor Object Reference") (OtherComp :type "PrimitiveComponent Object Reference") (OtherBodyIndex :type Integer) (bFromSweep :type Boolean) (SweepResult :type "HitResult Structure (by ref)"))
  (bind _asplayer_bp (cast `/Game/PlayerCharacter/Player_BP` OtherActor))
  (`GameplayStatics.ApplyDamage` _asplayer_bp 1.0))

(fn `UserConstructionScript`
  (bind _interptomovement (`self.InterpToMovement`))
  (set `InterpToMovementComponent.ControlPoints` (`|MakeArray` (make `InterpControlPoint` (`self.Location 1`)) (make `InterpControlPoint` (`self.Loccation 2`))) _interptomovement)
  (set `InterpToMovementComponent.Duration` (`self.Speed`) _interptomovement))