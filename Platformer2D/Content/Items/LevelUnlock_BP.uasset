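; LevelUnlock_BP is a level exit trigger that unlocks a level and travels to a named level.
; When Player_BP overlaps its box, it marks LevelNumber as true in the Levels array of the player's save object and saves it to a fixed slot.
; It then shows the Fade_WB widget, waits briefly and opens LevelName.
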(event `self.Box.OnComponentBeginOverlap`
  (params (OverlappedComponent :type "PrimitiveComponent Object Reference") (OtherActor :type "Actor Object Reference") (OtherComp :type "PrimitiveComponent Object Reference") (OtherBodyIndex :type Integer) (bFromSweep :type Boolean) (SweepResult :type "HitResult Structure (by ref)"))
  (bind _asplayer_bp (cast `/Game/PlayerCharacter/Player_BP` OtherActor))
  (bind _as_player_save (`/Game/PlayerCharacter/Player_BP.As Player Save` _asplayer_bp))
  (`KismetArrayLibrary.Array_Set` (`/Game/PlayerCharacter/PlayerSave.Levels` _as_player_save) (`self.levelNumber`) true)
  (`GameplayStatics.SaveGameToSlot` _as_player_save "1")
  (bind _returnvalue (`|CreateWidget` "/Game/WidgetBluePrints/Fade_WB.Fade_WB_C"))
  (`UserWidget.AddToViewport` _returnvalue 0)
  (`KismetSystemLibrary.Delay` 1.0)
  (`GameplayStatics.OpenLevel` (`self.Level Name`)))

(fn `UserConstructionScript`)