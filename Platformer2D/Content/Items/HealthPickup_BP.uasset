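; Health pickup actor that restores health to the player when touched.
; When an overlap with its sphere begins, it casts the other actor to Player_BP and acts only if that player is below MaxHealth.
; It adds HealthToGive clamped to the maximum, passes the truncated pickup amount to the player's HUD UpdateHealth, then destroys itself.
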(event `self.Sphere.OnComponentBeginOverlap`
  (params (OverlappedComponent :type "PrimitiveComponent Object Reference") (OtherActor :type "Actor Object Reference") (OtherComp :type "PrimitiveComponent Object Reference") (OtherBodyIndex :type Integer) (bFromSweep :type Boolean) (SweepResult :type "HitResult Structure (by ref)"))
  (bind _asplayer_bp (cast `/Game/PlayerCharacter/Player_BP` OtherActor))
  (bind _output_get (set `self.As Player BP` _asplayer_bp))
  (bind _health (`/Game/PlayerCharacter/Player_BP.health` _output_get))
  (bind _max_health (`/Game/PlayerCharacter/Player_BP.Max Health` _output_get))
  (if (< _health _max_health)
    (set `/Game/PlayerCharacter/Player_BP.health` (`KismetMathLibrary.FClamp` (+ _health (`self.healthToGive`)) 1.0 _max_health) _output_get)
    (`/Game/WidgetBluePrints/PlayerHud_WB.Update Health` (`/Game/PlayerCharacter/Player_BP.hudRef` _output_get) (`KismetMathLibrary.FTrunc` (`self.healthToGive`)))
    (`self.K2_DestroyActor`)))

(fn `UserConstructionScript`)