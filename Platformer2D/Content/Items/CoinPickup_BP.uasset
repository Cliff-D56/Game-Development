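; Coin pickup actor that a Player_BP collects by overlapping its sphere.
; Each pickup adds a coin, clamped to the player's MaxCoins.
; The coin that would reach the maximum instead grants an extra life and resets the count to zero.
; The player's HUD reference refreshes the lives and coin displays, then the pickup destroys itself.
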(event `self.Sphere.OnComponentBeginOverlap`
  (params (OverlappedComponent :type "PrimitiveComponent Object Reference") (OtherActor :type "Actor Object Reference") (OtherComp :type "PrimitiveComponent Object Reference") (OtherBodyIndex :type Integer) (bFromSweep :type Boolean) (SweepResult :type "HitResult Structure (by ref)"))
  (bind _hudref (`/Game/PlayerCharacter/Player_BP.hudRef` (`self.As Player BP`)))
  (bind _asplayer_bp (cast `/Game/PlayerCharacter/Player_BP` OtherActor))
  (bind _output_get (set `self.As Player BP` _asplayer_bp))
  (bind _coins (`/Game/PlayerCharacter/Player_BP.coins` _output_get))
  (bind _maxcoins (`/Game/PlayerCharacter/Player_BP.maxCoins` _output_get))
  (if (== _coins (- _maxcoins 1))
    (bind _result (`/Engine/EditorBlueprintResources/StandardMacros.IncrementFloat` (`/Game/PlayerCharacter/Player_BP.lives` _output_get))
      (:`  `
        (set `/Game/PlayerCharacter/Player_BP.lives` _result _output_get)
        (`/Game/WidgetBluePrints/PlayerHud_WB.UpdateLives` _hudref)
        (set `/Game/PlayerCharacter/Player_BP.coins` 0 _output_get)))
    (else
      (set `/Game/PlayerCharacter/Player_BP.coins` (`KismetMathLibrary.Clamp` (+ _coins 1) 1 _maxcoins) _output_get)))
  (`/Game/WidgetBluePrints/PlayerHud_WB.UpdateCoins` _hudref)
  (`self.K2_DestroyActor`))

(fn `UserConstructionScript`)