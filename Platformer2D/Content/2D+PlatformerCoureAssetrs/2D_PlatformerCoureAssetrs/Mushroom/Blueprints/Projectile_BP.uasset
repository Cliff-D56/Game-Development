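; Mushroom enemy projectile actor for a 2D platformer that damages the player on contact.
; When its Sphere begins overlapping the player character, it applies one point of damage and switches its Paper2D flipbook to the explosion animation.
; It waits for that flipbook's length, then destroys itself; overlaps with other actors are ignored.
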(event `self.Sphere.OnComponentBeginOverlap`
  (params (OverlappedComponent :type "PrimitiveComponent Object Reference") (OtherActor :type "Actor Object Reference") (OtherComp :type "PrimitiveComponent Object Reference") (OtherBodyIndex :type Integer) (bFromSweep :type Boolean) (SweepResult :type "HitResult Structure (by ref)"))
  (if (== OtherActor (`GameplayStatics.GetPlayerCharacter` 0))
    (`GameplayStatics.ApplyDamage` (`GameplayStatics.GetPlayerCharacter` 0) 1.0)
    (`PaperFlipbookComponent.SetFlipbook` (`self.PaperFlipbook`) "/Game/2D+PlatformerCoureAssetrs/2D_PlatformerCoureAssetrs/Mushroom/Flipbooks/ProjectileExploder/MushroomProjectileExplosion.MushroomProjectileExplosion")
    (`KismetSystemLibrary.Delay` (`PaperFlipbookComponent.GetFlipbookLength` (`self.PaperFlipbook`)))
    (`self.K2_DestroyActor`)))

(fn `UserConstructionScript`)