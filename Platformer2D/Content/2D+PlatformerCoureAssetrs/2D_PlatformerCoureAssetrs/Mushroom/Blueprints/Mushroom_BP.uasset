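; Mushroom ranged enemy for a 2D platformer that turns to face the player each tick while alive.
; The player entering its Box trigger starts a looping timer that plays the Attack animation while grounded; leaving clears it.
; A separate SpawnProjectile event fires Projectile_BP from the spawn point.
; Damage updates a widget health bar, then either launches the mushroom with a hit animation or plays death and destroys it after a delay.
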(event `self.ReceiveBeginPlay`
  (set `self.maxHealth` (`self.Health`))
  (bind _asranged_enemy_health_bar (cast `/Game/WidgetBluePrints/RangedEnemyHealthBar` (`WidgetComponent.GetWidget` (`self.HealthBar`))))
  (bind _output_get (set `self.As Ranged Enemy Health Bar` _asranged_enemy_health_bar))
  (set `/Game/WidgetBluePrints/RangedEnemyHealthBar.mushroomRef` self _output_get))

(event `self.ReceiveTick`
  (params (DeltaSeconds :type "Float (single-precision)"))
  (`self.HandleRotation`))

(event `self.ReceiveAnyDamage`
  (params (Damage :type "Float (single-precision)") (DamageType :type "DamageType Object Reference") (InstigatedBy :type "Controller Object Reference") (DamageCauser :type "Actor Object Reference"))
  (bind _returnvalue_x (`KismetMathLibrary.BreakVector` (`KismetMathLibrary.GetDirectionUnitVector` (`self.K2_GetActorLocation` DamageCauser) (`self.K2_GetActorLocation`))))
  ;[1 1 1] Handles Enemy Damage
  (bind _output_get (set `self.Health` (- (`self.Health`) Damage)))
  (`/Game/WidgetBluePrints/RangedEnemyHealthBar.updateHealthbar` (`self.As Ranged Enemy Health Bar`))
  (set `self.enemyDamaged` true)
  (if (<= _output_get 0.0)
    (`PaperZDAnimInstance.JumpToNode` (`PaperZDAnimationComponent.AnimInstance` (`self.AnimationComponent`)) "Mushroom Death" "None")
    (`SceneComponent.SetVisibility` (`self.HealthBar`) false false)
    (set `self.isDead?` true)
    (`PrimitiveComponent.SetCollisionProfileName` (`self.CapsuleComponent`) "OverlapOnlyPawn" true)
    (`KismetSystemLibrary.Delay` 3.0)
    (`self.K2_DestroyActor`)
    (else
      (`self.LaunchCharacter` (`KismetMathLibrary.MakeVector` (* (select `bool` (< _returnvalue_x 0.0) :`false` -1.0 :`true` 1.0) -800.0) 0.0 100.0) true true)
      (`PaperZDAnimInstance.JumpToNode` (`PaperZDAnimationComponent.AnimInstance` (`self.AnimationComponent`)) "Damaged" "None")
      (`SceneComponent.SetVisibility` (`self.HealthBar`) true false)
      (`KismetSystemLibrary.RetriggerableDelay` 1.0)
      (set `self.enemyDamaged` false))))

(event `HandleRotation`
  (bind _returnvalue_x (`KismetMathLibrary.BreakVector` (`KismetMathLibrary.GetDirectionUnitVector` (`self.K2_GetActorLocation` (`GameplayStatics.GetPlayerCharacter` 0)) (`self.K2_GetActorLocation`))))
  (if (`self.isDead?`)
    _
    (elif (< _returnvalue_x 0.0)
      (`self.K2_SetActorRotation` (struct))
      (else
        (`self.K2_SetActorRotation` (struct :`Yaw` 180.0))))))

(event `self.Box.OnComponentBeginOverlap`
  (params (OverlappedComponent :type "PrimitiveComponent Object Reference") (OtherActor :type "Actor Object Reference") (OtherComp :type "PrimitiveComponent Object Reference") (OtherBodyIndex :type Integer) (bFromSweep :type Boolean) (SweepResult :type "HitResult Structure (by ref)"))
  (if (== OtherActor (`GameplayStatics.GetPlayerCharacter` 0))
    (set `self.attackMode` true)
    (bind _returnvalue (`KismetSystemLibrary.K2_SetTimerDelegate` (delegate `mushroomAttack`) 1.0 true))
    (set `self.AttackEvent` _returnvalue)))

(event `mushroomAttack`
  (if (not (or (`self.isDead?`) (`NavMovementComponent.IsFalling` (`self.CharacterMovement`))))
    (`PaperZDAnimInstance.JumpToNode` (`PaperZDAnimationComponent.AnimInstance` (`self.AnimationComponent`)) "Attack" "None")))

(event `SpawnProjectile`
  (`|SpawnActorFromClass` "/Game/2D+PlatformerCoureAssetrs/2D_PlatformerCoureAssetrs/Mushroom/Blueprints/Projectile_BP.Projectile_BP_C" (`KismetMathLibrary.MakeTransform` (`SceneComponent.K2_GetComponentLocation` (`self.SpawnPoint`)) (`self.K2_GetActorRotation`)) "Undefined" "MultiplyWithRoot" null null))

(event `self.Box.OnComponentEndOverlap`
  (params (OverlappedComponent :type "PrimitiveComponent Object Reference") (OtherActor :type "Actor Object Reference") (OtherComp :type "PrimitiveComponent Object Reference") (OtherBodyIndex :type Integer))
  (if (== OtherActor (`GameplayStatics.GetPlayerCharacter` 0))
    (set `self.attackMode` false)
    (`KismetSystemLibrary.K2_ClearAndInvalidateTimerHandle` (`self.attackEvent`))))

(fn `UserConstructionScript`)