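; Skeleton enemy for a 2D platformer that patrols back and forth along the X axis, turning at obstacles and ledges.
; Every tick it faces its MovementDirection, adds movement input and runs two line traces that ignore the player: forward for obstacles, forward-down for missing ground.
; Both feed one DoOnce that stops the walk, waits WaitTime, restores speed, reverses direction and resets.
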(event `self.ReceiveBeginPlay`
  ;[1 1 1] Standardized Walk Speed Check
  (set `CharacterMovementComponent.MaxWalkSpeed` (`self.Max Walk Speed`) (`self.CharacterMovement`)))

(event `self.ReceiveTick`
  (params (DeltaSeconds :type "Float (single-precision)"))
  ;[1 1 1] Constant Rotation and Movement Check
  (`self.HandleRotation`)
  (`self.HandleMovement`))

(event `HandleRotation`
  ;[1 1 1] Enemy Rotation
  (if (> (`self.MovementDirection`) 0.0)
    (`self.K2_SetActorRotation` (struct))
    (else
      (`self.K2_SetActorRotation` (struct :`Yaw` 180.0)))))

(event `HandleMovement`
  (bind _returnvalue (`self.K2_GetActorLocation`))
  (bind _returnvalue_2 (`self.K2_GetActorLocation`))
  ;[1 1 1] Enemy Movement and Detection
  (`self.AddMovementInput` (1.0 0.0 0.0) (`self.MovementDirection`))
  (`|ExecutionSequence`
    (:`then_0`
      (bind (_outhit _returnvalue_3) (`KismetSystemLibrary.LineTraceSingleForObjects` _returnvalue (+ _returnvalue (* (`self.GetActorForwardVector`) (100.0 0.0 0.0))) (`|MakeArray` "ObjectTypeQuery1" "ObjectTypeQuery2" "ObjectTypeQuery3" :!type "EObjectTypeQuery Enum") false (`|MakeArray` (`GameplayStatics.GetPlayerCharacter` 0) :!type "Actor Object Reference")))
      ;;[1 1 1] Sets Walkspeed to 0 THEN a Delay using Wait time Variable Sets Walk speed back to Max Walk speed THEN Movement Direction is reversed before the loop resets waiting for another collision.
      (if _returnvalue_3
        (`/Engine/EditorBlueprintResources/StandardMacros.DoOnce` false :!label _label
          (:`Completed`
            (set `CharacterMovementComponent.MaxWalkSpeed` 0.0 (`self.CharacterMovement`))
            (`KismetSystemLibrary.Delay` (`self.WaitTime`))
            (set `CharacterMovementComponent.MaxWalkSpeed` (`self.Max Walk Speed`) (`self.CharacterMovement`))
            (set `self.MovementDirection` (* (`self.MovementDirection`) -1.0))
            (goto _label :!via `Reset`)))))
    (:`then_1`
      ;[1 1 1] Gets the Actor location and has the forward vector line 100 units below Z axis and 100 units forward on the X axis, the line trace is always checking for ground so its always true, when its not true there is no ground and it will immediately go to reverse player rotation
      (bind (_outhit_2 _returnvalue_4) (`KismetSystemLibrary.LineTraceSingleForObjects` _returnvalue_2 (+ (- _returnvalue_2 (0.0 0.0 100.0)) (* (`self.GetActorForwardVector`) (100.0 0.0 0.0))) (`|MakeArray` "ObjectTypeQuery1" "ObjectTypeQuery2" "ObjectTypeQuery3" :!type "EObjectTypeQuery Enum") false (`|MakeArray` (`GameplayStatics.GetPlayerCharacter` 0) :!type "Actor Object Reference") "ForDuration"))
      (if (not _returnvalue_4)
        (goto _label)))))

(fn `UserConstructionScript`)