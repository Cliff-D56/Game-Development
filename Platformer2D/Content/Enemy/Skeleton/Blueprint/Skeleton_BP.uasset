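; Skeleton enemy character for a side-on game that patrols along X, pausing and reversing at obstacles or ledges found by line traces.
; The player entering its box stops patrol and starts a looping attack timer, with the animation's Attack event tracing to apply damage.
; Damage updates a healthbar widget and triggers knockback or death through animation node jumps, then destroys the dead skeleton after a delay.
; Distance-based player detection is unfinished and never called.
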(event `self.ReceiveBeginPlay`
  ;[1 1 1] Standardized Walk Speed Check
  (set `CharacterMovementComponent.MaxWalkSpeed` (`self.Max Walk Speed`) (`self.CharacterMovement`))
  (set `self.maxHealth` (`self.Health`))
  (bind _asenemy_healthbar_wb (cast `/Game/WidgetBluePrints/EnemyHealthbar_WB` (`WidgetComponent.GetWidget` (`self.Widget`))))
  (set `/Game/WidgetBluePrints/EnemyHealthbar_WB.skeletonRef` self _asenemy_healthbar_wb)
  (set `self.As Enemy Healthbar WB` _asenemy_healthbar_wb))

(event `self.ReceiveTick`
  (params (DeltaSeconds :type "Float (single-precision)"))
  ;[1 1 1] Constant Rotation and Movement Check
  (`self.HandleRotation`)
  (`self.HandleMovement`))

(event `HandleRotation`
  ;[1 1 1] Enemy Rotation
  (if (> (`self.MovementDirection`) 0.0)
    (`self.K2_SetActorRotation` (struct))
    (else
      (`self.K2_SetActorRotation` (struct :`Yaw` 180.0)))))

(event `HandleMovement`
  (bind _returnvalue (`self.K2_GetActorLocation`))
  (bind _returnvalue_2 (`self.K2_GetActorLocation`))
  ;[1 1 1] Enemy Movement and Detection
  (if (not (or (`self.isDead?`) (`self.enemyDamaged`) (`NavMovementComponent.IsFalling` (`self.CharacterMovement`)) (`self.attackMode`)))
    (`self.AddMovementInput` (1.0 0.0 0.0) (`self.MovementDirection`))
    (`|ExecutionSequence`
      (:`then_0`
        (bind (_outhit _returnvalue_3) (`KismetSystemLibrary.LineTraceSingleForObjects` _returnvalue (+ _returnvalue (* (`self.GetActorForwardVector`) (100.0 0.0 0.0))) (`|MakeArray` "ObjectTypeQuery1" "ObjectTypeQuery2" "ObjectTypeQuery3" :!type "EObjectTypeQuery Enum") false (`|MakeArray` (`GameplayStatics.GetPlayerCharacter` 0) null :!type "Actor Object Reference")))
        ;;[1 1 1] Sets Walkspeed to 0 THEN a Delay using Wait time Variable Sets Walk speed back to Max Walk speed THEN Movement Direction is reversed before the loop resets waiting for another collision.
        (if _returnvalue_3
          (`/Engine/EditorBlueprintResources/StandardMacros.DoOnce` false :!label _label
            (:`Completed`
              (set `CharacterMovementComponent.MaxWalkSpeed` 0.0 (`self.CharacterMovement`))
              (`KismetSystemLibrary.Delay` (`self.WaitTime`))
              (set `CharacterMovementComponent.MaxWalkSpeed` (`self.Max Walk Speed`) (`self.CharacterMovement`))
              (set `self.MovementDirection` (* (`self.MovementDirection`) -1.0))
              (goto _label :!via `Reset`)))))
      (:`then_1`
        ;[1 1 1] Gets the Actor location and has the forward vector line 100 units below Z axis and 100 units forward on the X axis, the line trace is always checking for ground so its always true, when its not true there is no ground and it will immediately go to reverse player rotation
        (bind (_outhit_2 _returnvalue_4) (`KismetSystemLibrary.LineTraceSingleForObjects` _returnvalue_2 (+ (- _returnvalue_2 (0.0 0.0 100.0)) (* (`self.GetActorForwardVector`) (100.0 0.0 0.0))) (`|MakeArray` "ObjectTypeQuery1" "ObjectTypeQuery2" "ObjectTypeQuery3" :!type "EObjectTypeQuery Enum") false (`|MakeArray` (`GameplayStatics.GetPlayerCharacter` 0) :!type "Actor Object Reference")))
        (if (not _returnvalue_4)
          (goto _label))))))

(event `self.ReceiveAnyDamage`
  (params (Damage :type "Float (single-precision)") (DamageType :type "DamageType Object Reference") (InstigatedBy :type "Controller Object Reference") (DamageCauser :type "Actor Object Reference"))
  (bind _returnvalue_x (`KismetMathLibrary.BreakVector` (`KismetMathLibrary.GetDirectionUnitVector` (`self.K2_GetActorLocation` DamageCauser) (`self.K2_GetActorLocation`))))
  (bind _returnvalue (select `bool` (< _returnvalue_x 0.0) :`false` -1.0 :`true` 1.0))
  ;[1 1 1] Handles Enemy Damage
  (bind _output_get (set `self.Health` (- (`self.Health`) Damage)))
  (`/Game/WidgetBluePrints/EnemyHealthbar_WB.updateHealthbar` (`self.As Enemy Healthbar WB`))
  (set `self.enemyDamaged` true)
  (set `self.MovementDirection` _returnvalue)
  (if (<= _output_get 0.0)
    (`PaperZDAnimInstance.JumpToNode` (`PaperZDAnimationComponent.AnimInstance` (`self.AnimationComponent`)) (`self.DeathJumpNode`) "None")
    (`SceneComponent.SetVisibility` (`self.Widget`) false false)
    (set `self.isDead?` true)
    (`PrimitiveComponent.SetCollisionProfileName` (`self.CapsuleComponent`) "OverlapOnlyPawn" true)
    (`KismetSystemLibrary.Delay` 3.0)
    (`self.K2_DestroyActor`)
    (else
      (`self.LaunchCharacter` (`KismetMathLibrary.MakeVector` (* _returnvalue -800.0) 0.0 100.0) true true)
      (`PaperZDAnimInstance.JumpToNode` (`PaperZDAnimationComponent.AnimInstance` (`self.AnimationComponent`)) (`self.DamagedJumpNode`) "None")
      (`SceneComponent.SetVisibility` (`self.Widget`) true false)
      (`KismetSystemLibrary.RetriggerableDelay` 1.0)
      (set `self.enemyDamaged` false))))

(event `self.Box.OnComponentBeginOverlap`
  (params (OverlappedComponent :type "PrimitiveComponent Object Reference") (OtherActor :type "Actor Object Reference") (OtherComp :type "PrimitiveComponent Object Reference") (OtherBodyIndex :type Integer) (bFromSweep :type Boolean) (SweepResult :type "HitResult Structure (by ref)"))
  ;[1 1 1] Sets Enemy to Attack Mode if Pawn enters Box Overlap
  (if (== OtherActor (`GameplayStatics.GetPlayerCharacter` 0))
    (set `self.attackMode` true)
    (bind _returnvalue (`KismetSystemLibrary.K2_SetTimerDelegate` (delegate `skeletonAttack`) 1.0 true))
    (set `self.attackEvent` _returnvalue)))

(event `skeletonAttack`
  ;[1 1 1] Sets Enemy to Attack Mode if Pawn enters Box Overlap
  (if (not (`self.isDead?`))
    (`PaperZDAnimInstance.JumpToNode` (`PaperZDAnimationComponent.AnimInstance` (`self.AnimationComponent`)) (`self.Attack Jump Node`) "None")))

(event `Attack`
  (bind _returnvalue (`self.K2_GetActorLocation`))
  ;[1 1 1] Handles Attack Notify on Enemy Animation
  (bind _outhit (`KismetSystemLibrary.LineTraceSingleForObjects` _returnvalue (+ _returnvalue (* (150.0 0.0 0.0) (`self.GetActorForwardVector`))) (`|MakeArray` "ObjectTypeQuery3" :!type "EObjectTypeQuery Enum")))
  (bind (_bblockinghit _binitialoverlap _time _distance _location _impactpoint _normal _impactnormal _physmat _hitactor) (`GameplayStatics.BreakHitResult` _outhit))
  (if (== _hitactor (`GameplayStatics.GetPlayerCharacter` 0))
    (`GameplayStatics.ApplyDamage` _hitactor 1.0)))

(event `self.Box.OnComponentEndOverlap`
  (params (OverlappedComponent :type "PrimitiveComponent Object Reference") (OtherActor :type "Actor Object Reference") (OtherComp :type "PrimitiveComponent Object Reference") (OtherBodyIndex :type Integer))
  ;[1 1 1] Upon Pawn Leaving Overlap Attack Mode is switched off
  (if (== OtherActor (`GameplayStatics.GetPlayerCharacter` 0))
    (set `self.attackMode` false)
    (`KismetSystemLibrary.K2_ClearAndInvalidateTimerHandle` (`self.attackEvent`))))

(event `Enemy Detection`
  (bind _returnvalue_x (`KismetMathLibrary.BreakVector` (`KismetMathLibrary.GetDirectionUnitVector` (`self.K2_GetActorLocation`) (`self.K2_GetActorLocation` (`GameplayStatics.GetPlayerCharacter` 0)))))
  (if (<= (`KismetMathLibrary.Vector_Distance` (`self.K2_GetActorLocation`) (`self.K2_GetActorLocation` (`GameplayStatics.GetPlayerCharacter` 0))) (`self.detectionRange`))
    (set `self.playerClose?` true)
    (else
      (set `self.playerClose?` false)))
  (`KismetSystemLibrary.PrintString` (`KismetStringLibrary.Conv_BoolToString` (`self.playerClose?`)))
  (if (`self.playerClose?`)
    (set `self.MovementDirection` (select `bool` (< _returnvalue_x 0.0) :`false` 1.0 :`true` -1.0))))

(fn `UserConstructionScript`)